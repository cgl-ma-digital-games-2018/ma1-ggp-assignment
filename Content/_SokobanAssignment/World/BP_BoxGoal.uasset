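; BP_BoxGoal is a Sokoban goal that detects when a BP_MovableBox sits on it.
; Its Box overlap events recolor the goal's PointLight and call LightOn or LightOff dispatchers, with comments indicating a linked wall light.
; On entry it also asks BP_SokobanAssignmentGameMode to check the win condition.
; On exit it restores the starting color without rechecking.
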(event `self.ReceiveBeginPlay`)

(event `self.Box.OnComponentBeginOverlap`
  (params (OverlappedComponent :type "PrimitiveComponent Object Reference") (OtherActor :type "Actor Object Reference") (OtherComp :type "PrimitiveComponent Object Reference") (OtherBodyIndex :type Integer) (bFromSweep :type Boolean) (SweepResult :type "HitResult Structure (by ref)"))
  ;[1 1 1] Change Colour on ground and wall light
  (cast `/Game/_SokobanAssignment/Props/BP_MovableBox` OtherActor)
  (`LightComponent.SetLightColor` (`self.PointLight`) (struct :`G` 0.061501 :`B` 1.0 :`A` 1.0) true)
  (`self.LightOn`)
  (bind _asbp_sokoban_assignment_game_mode (cast `/Game/_SokobanAssignment/Core/GameModes/BP_SokobanAssignmentGameMode` (`GameplayStatics.GetGameMode`))
    (:`then`
      (bind _output_get (set `self.CurrentGameMode` _asbp_sokoban_assignment_game_mode))
      (`SokobanAssignmentGameMode.CheckForWinCondition` _output_get))
    (:`CastFailed`
      (`KismetSystemLibrary.PrintString` "Cast failed!"))))

(event `self.Box.OnComponentEndOverlap`
  (params (OverlappedComponent :type "PrimitiveComponent Object Reference") (OtherActor :type "Actor Object Reference") (OtherComp :type "PrimitiveComponent Object Reference") (OtherBodyIndex :type Integer))
  ;[1 1 1] Reset Colour to Starting Colour for both
  (cast `/Game/_SokobanAssignment/Props/BP_MovableBox` OtherActor)
  (`LightComponent.SetLightColor` (`self.PointLight`) (struct :`R` 0.59 :`G` 1.0 :`B` 0.9 :`A` 1.0) true)
  (`self.LightOff`))

(fn `UserConstructionScript`)